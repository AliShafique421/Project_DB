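; BP_ScreenTest is a test Blueprint that checks whether its actor's location lands inside a centered screen frame.
; Shortly after BeginPlay, CalculateFrameWidth sizes the frame once as percentages of the viewport.
; Each Tick, IsVisibleToCamera projects the location for player 0 and compares it to the frame bounds, without occlusion checks.
; Tick discards the result, and the projection's success flag is ignored.
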(event EventTick
  (params (DeltaSeconds :type Float%20%28single-precision%29))
  (CallFunction|IsVisibletoCamera))

(event EventBeginPlay
  (Utilities|FlowControl|Delay 0.1)
  (CallFunction|CalculateFrameWidth))

(fn ConstructionScript)

(fn IsVisibletoCamera
  (bind _returnvalue (Viewport|GetViewportSize))
  (bind _framewidthy (Variables|Default|GetFrameWidthY))
  (bind _framewidthx (Variables|Default|GetFrameWidthX))
  (bind _returnvalue_2 (* _framewidthx 0.5))
  (bind _returnvalue_3 (* _framewidthy 0.5))
  (LocalVariables|SetScreenPosition (.ScreenPosition (Class|GameplayStatics|ProjectWorldtoScreen (Game|GetPlayerController 0) (Transformation|GetActorLocation) false)))
  (LocalVariables|SetScreenCenterX (* (.x _returnvalue) 0.5))
  (LocalVariables|SetScreenCenterY (* (.y _returnvalue) 0.5))
  (LocalVariables|SetMinX (- (LocalVariables|GetScreenCenterX) _returnvalue_2))
  (LocalVariables|SetMaxX (+ (LocalVariables|GetScreenCenterX) _returnvalue_2))
  (LocalVariables|SetMinY (- (LocalVariables|GetScreenCenterY) _returnvalue_3))
  (LocalVariables|SetMaxY (+ (LocalVariables|GetScreenCenterY) _returnvalue_3))
  (return (Math|Boolean|ANDBoolean (>= (.x (LocalVariables|GetScreenPosition)) (LocalVariables|GetMinX)) (<= (.x (LocalVariables|GetScreenPosition)) (LocalVariables|GetMaxX)) (>= (.y (LocalVariables|GetScreenPosition)) (LocalVariables|GetMinY)) (<= (.y (LocalVariables|GetScreenPosition)) (LocalVariables|GetMaxY)))))

(fn CalculateFrameWidth
  (bind _returnvalue (Viewport|GetViewportSize))
  (Variables|Default|SetFrameWidthX (/ (* (.x _returnvalue) (Variables|Default|GetFramePercentageX)) 1e+02))
  (Variables|Default|SetFrameWidthY (/ (* (.y _returnvalue) (Variables|Default|GetFramePercentageY)) 1e+02)))