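; Player controller blueprint for an ALS-based character setup.
; On possession it casts the player camera manager to ALS_PlayerCameraManager and hands it the possessed pawn through OnPossess.
; It implements a debug info interface function that returns its debug state: focus character, debug view, HUD, trace, shape, layer color, slomo and character info settings.
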(event EventPossess
  (params (PossessedPawn :type Pawn%20Object%20Reference))
  (bind _asals_player_camera_manager (Utilities|Casting|CastToALS_PlayerCameraManager (Variables|Default|GetPlayerCameraManager)))
  (Default|OnPossess _asals_player_camera_manager PossessedPawn))

(fn ConstructionScript)

(fn BPIGetDebugInfo
  (return (Variables|Debug|GetDebugFocusCharacter) (Variables|Debug|GetDebugView) (Variables|Debug|GetShowHUD) (Variables|Debug|GetShowTraces) (Variables|Debug|GetShowDebugShapes) (Variables|Debug|GetShowLayerColors) (Variables|Debug|GetSlomo) (Variables|Debug|GetShowCharacterInfo)))