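; Actor component for the phone system's bank and market, holding the player's money and a timestamped transaction list.
; Purchases deduct item fees from a shopping DataTable; SendMoney routes transfers to bot dispatchers or, via a server event, to another player's component found by phone number.
; Incoming player or delayed bot payments credit money, log a transaction, and either refresh the open bank app or show a phone notification.
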(event Custom|BuyItem
  (params (ItemRow :type Name))
  ;[0 0 0] Buy Item
  (bind _returnvalue (Utilities|GetDataTableRow "/Game/PhoneSystem/Data/BankShop/DT_ShoppingItemList.DT_ShoppingItemList" ItemRow)
    (:then
      (Variables|Settings|SetCurrentMoney (- (Variables|Settings|GetCurrentMoney) (.ItemFee (Utilities|Struct|BreakS_ShoppingItemDetails _returnvalue))))
      (CallFunction|AddNewTransactions "Market" (* (.ItemFee (Utilities|Struct|BreakS_ShoppingItemDetails _returnvalue)) -1.0) (.ItemIcon (Utilities|Struct|BreakS_ShoppingItemDetails _returnvalue)))
      (Default|CallItemAdded _returnvalue)
      (bind _foundwidgets (Widget|GetAllWidgetsOfClass "/Game/PhoneSystem/UI/Apps/WBP_MarketApp.WBP_MarketApp_C" false))
      (Utilities|IsValid (Utilities|Array|Get(acopy) _foundwidgets)
        (:Is%20Valid
          (Default|UpdateCurrentMoney (Utilities|Array|Get(acopy) _foundwidgets)))))))

(event Custom|ForwardMoneyTransfer_Server
  (params (ReceiverNumber :type String) (SenderNumber :type String) (Amount :type Float%20%28double-precision%29))
  ;[0 0 0] Forward Money Transfer
  (CallFunction|ReceiveMoneyOwningClient (Actor|GetComponentbyClass (CallFunction|FindPlayerbyNumber ReceiverNumber) "AC_BankAndShop_C") SenderNumber Amount))

(event Custom|ReceiveMoneyFromBot
  (params (Amount :type Float%20%28double-precision%29) (BotName :type String) (BotPicture :type Texture%202D%20Object%20Reference) (SendDelay :type Float%20%28double-precision%29))
  ;[0 0 0] Bot Send Money to player
  (Utilities|FlowControl|Delay SendDelay)
  (Variables|Settings|SetCurrentMoney (+ Amount (Variables|Settings|GetCurrentMoney)))
  (CallFunction|AddNewTransactions (Utilities|Text|ToText(String) BotName) Amount BotPicture)
  (Audio|PlaySound2D "/Game/PhoneSystem/Sound/SW_Cash.SW_Cash" 1.0 1.0 0.0 0 0)
  (bind _foundwidgets (Widget|GetAllWidgetsOfClass "/Game/PhoneSystem/UI/WBP_MainPhone.WBP_MainPhone_C" false))
  (Utilities|IsValid (Utilities|Array|Get(acopy) _foundwidgets)
    (:Is%20Valid
      (bind _aswbp_bank_app (Utilities|Casting|CastToWBP_BankApp (Variables|/Game/PhoneSystem/UI/WBP_MainPhone.WBP_MainPhone_C|GetCurrentAppRef (Utilities|Array|Get(acopy) _foundwidgets)))
        (:then
          (if (== (Class|WidgetSwitcher|GetActiveWidgetIndex (Variables|/Game/PhoneSystem/UI/Apps/WBP_BankApp.WBP_BankApp_C|GetWidgetSwitcher_0 _aswbp_bank_app)) 1)
            (Default|UpdateDetails _aswbp_bank_app)))
        (:CastFailed
          (Default|NotifyMessage (Variables|/Game/PhoneSystem/UI/WBP_MainPhone.WBP_MainPhone_C|GetMainScreenRef (Utilities|Array|Get(acopy) _foundwidgets)) "System" "Money Received" "-1"))))))

(event Custom|ReceiveMoney_OwningClient
  (params (SenderNumber :type String) (Amount :type Float%20%28double-precision%29))
  (bind _returnvalue (CallFunction|FindPlayerStatefromNumber SenderNumber))
  (bind _profiledetails (Variables|/Game/PhoneSystem/Blueprint/Core/BP_PhonePlayerState.BP_PhonePlayerState_C|GetProfileDetails _returnvalue))
  (bind (_name _profileicon) (Utilities|Struct|BreakS_ProfileDetails _profiledetails))
  ;[0 0 0] Other Player Send Money
  (Variables|Settings|SetCurrentMoney (+ Amount (Variables|Settings|GetCurrentMoney)))
  (CallFunction|AddNewTransactions (Utilities|Text|ToText(String) _name) Amount _profileicon)
  (bind _foundwidgets (Widget|GetAllWidgetsOfClass "/Game/PhoneSystem/UI/WBP_MainPhone.WBP_MainPhone_C" false))
  (Utilities|IsValid (Utilities|Array|Get(acopy) _foundwidgets)
    (:Is%20Valid
      (bind _aswbp_bank_app (Utilities|Casting|CastToWBP_BankApp (Variables|/Game/PhoneSystem/UI/WBP_MainPhone.WBP_MainPhone_C|GetCurrentAppRef (Utilities|Array|Get(acopy) _foundwidgets)))
        (:then
          (if (== (Class|WidgetSwitcher|GetActiveWidgetIndex (Variables|/Game/PhoneSystem/UI/Apps/WBP_BankApp.WBP_BankApp_C|GetWidgetSwitcher_0 _aswbp_bank_app)) 1)
            (Default|UpdateDetails _aswbp_bank_app)))
        (:CastFailed
          (Default|NotifyMessage (Variables|/Game/PhoneSystem/UI/WBP_MainPhone.WBP_MainPhone_C|GetMainScreenRef (Utilities|Array|Get(acopy) _foundwidgets)) "System" "Money Received" "-1"))))))

(fn AddNewTransactions
  (params (ShopName :type Text) (Fee :type Float%20%28double-precision%29) (ShopImage :type Texture%202D%20Object%20Reference))
  (bind _returnvalue (Math|DateTime|Now))
  (bind (_year _month _day _hour _minute) (Math|DateTime|BreakDateTime _returnvalue))
  (bind _returnvalue_2 (Utilities|String|ToString(Integer) _minute))
  (bind _returnvalue_3 (Utilities|String|ToString(Integer) _hour))
  (Utilities|Array|Add (Variables|Settings|GetTransactionsList) (Utilities|Struct|MakeS_TransactionsDetails ShopName Fee (Utilities|Text|FormatText "{Hour}:{Minute}" (select (< _hour 10) (Utilities|String|Append "0" _returnvalue_3) _returnvalue_3) (select (< _minute 10) (Utilities|String|Append "0" _returnvalue_2) _returnvalue_2)) ShopImage)))

(fn CanBuyItem
  (params (ItemRow :type Name))
  (bind _returnvalue (Utilities|GetDataTableRow "/Game/PhoneSystem/Data/BankShop/DT_ShoppingItemList.DT_ShoppingItemList" ItemRow)
    (:then
      (return (>= (Variables|Settings|GetCurrentMoney) (.ItemFee (Utilities|Struct|BreakS_ShoppingItemDetails _returnvalue)))))))

(fn SendMoney
  (params (ReceiverNumber :type String) (SenderNumber :type String) (Amount :type Float%20%28double-precision%29))
  (if (Math|Boolean|ANDBoolean (not (Utilities|Array|IsEmpty ReceiverNumber)) (> Amount 0.0) (> (Variables|Settings|GetCurrentMoney) Amount))
    (bind _foundwidgets (Widget|GetAllWidgetsOfClass "/Game/PhoneSystem/UI/WBP_MainPhone.WBP_MainPhone_C" false))
    (Utilities|IsValid (Utilities|Array|Get(acopy) _foundwidgets)
      (:Is%20Valid
        (Variables|Settings|SetCurrentMoney (- (Variables|Settings|GetCurrentMoney) Amount))
        (if (.Find (Default|GetProfleDetails (Utilities|Array|Get(acopy) _foundwidgets) ReceiverNumber))
          (if (.IsBotProfile (Utilities|Struct|BreakS_ProfileDetails (.Details (Default|GetProfleDetails (Utilities|Array|Get(acopy) _foundwidgets) ReceiverNumber))))
            (Default|CallBotMoneyReceived ReceiverNumber Amount true)
            (CallFunction|AddNewTransactions (Utilities|Text|ToText(String) (.Name (Utilities|Struct|BreakS_ProfileDetails (.Details (Default|GetProfleDetails (Utilities|Array|Get(acopy) _foundwidgets) ReceiverNumber))))) (* Amount -1.0) (.ProfileIcon (Utilities|Struct|BreakS_ProfileDetails (.Details (Default|GetProfleDetails (Utilities|Array|Get(acopy) _foundwidgets) ReceiverNumber)))))
            (return true)
            (else
              (CallFunction|ForwardMoneyTransferServer ReceiverNumber SenderNumber Amount)
              (CallFunction|AddNewTransactions (Utilities|Text|ToText(String) (.Name (Utilities|Struct|BreakS_ProfileDetails (.Details (Default|GetProfleDetails (Utilities|Array|Get(acopy) _foundwidgets) ReceiverNumber))))) (* Amount -1.0) (.ProfileIcon (Utilities|Struct|BreakS_ProfileDetails (.Details (Default|GetProfleDetails (Utilities|Array|Get(acopy) _foundwidgets) ReceiverNumber)))))
              (return true)))
          (else
            (Default|CallBotMoneyReceived ReceiverNumber Amount false)
            (CallFunction|AddNewTransactions (Utilities|Text|ToText(String) ReceiverNumber) (* Amount -1.0) "/Game/PhoneSystem/Demo/Texture/ProfilePicture/T_UnkownUserWhite.T_UnkownUserWhite")
            (return true))))
      (:Is%20Not%20Valid
        (return false)))
    (else
      (return false))))

(fn FindPlayerbyNumber
  (params (ReceiverNumber :type String))
  (for _array_element (Variables|/Script/Engine.GameStateBase|GetPlayerArray (Game|GetGameState))
    (bind _asbp_phone_player_state (Utilities|Casting|CastToBP_PhonePlayerState _array_element))
    (if (Utilities|Enum|Equal(Enum) (Utilities|Struct|BreakS_ProfileDetails (Variables|/Game/PhoneSystem/Blueprint/Core/BP_PhonePlayerState.BP_PhonePlayerState_C|GetProfileDetails _asbp_phone_player_state)) ReceiverNumber)
      (return (PlayerState|GetPawn _asbp_phone_player_state)))))

(fn FindPlayerStatefromNumber
  (params (Number :type String))
  (for _array_element (Variables|/Script/Engine.GameStateBase|GetPlayerArray (Game|GetGameState))
    (bind _asbp_phone_player_state (Utilities|Casting|CastToBP_PhonePlayerState _array_element))
    (if (Utilities|Enum|Equal(Enum) (Utilities|Struct|BreakS_ProfileDetails (Variables|/Game/PhoneSystem/Blueprint/Core/BP_PhonePlayerState.BP_PhonePlayerState_C|GetProfileDetails _asbp_phone_player_state)) Number)
      (return _asbp_phone_player_state))))