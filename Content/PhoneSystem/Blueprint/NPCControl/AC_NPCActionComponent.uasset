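; NPC action component for the phone system, letting AI-controlled pawns walk to targets and send photos to the player's phone.
; It removes itself from player-controlled pawns.
; Movement resolves targets directly or by class, tag and index, retries on failure, loops in follow mode, and cancels through gates.
; Photos use a lazily created, tagged scene capture aimed by rotation or look-at, writing new render targets that are messaged to PlayerPhoneComponent.
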(event Custom|CancelSendTarget
  ;[0 0 0] Send Npc to Target
  (AI|Navigation|StopMovement (Variables|Default|GetAIController))
  (Utilities|FlowControl|Sequence
    (:then_0
      (Utilities|FlowControl|Gate false) ; enters at Close
    )
    (:then_1
      (Utilities|FlowControl|Gate false) ; enters at Close
    )))

(event Custom|TakePhoto
  (params (TargetLocation :type Vector) (TargetRotation :type Rotator) (TargetByRotation :type Boolean) (Delay :type Float%20%28single-precision%29) (TargetActor :type Actor%20Object%20Reference))
  (bind _output (CallFunction|GetSceneCapturer))
  (bind _playerphonecomponent (Variables|Default|GetPlayerPhoneComponent))
  (bind _npc_number (Variables|Default|GetNPC%20Number))
  (bind _receivedphoto (Variables|/Game/PhoneSystem/Blueprint/Component/AC_PhoneComponent.AC_PhoneComponent_C|GetReceivedPhoto _playerphonecomponent))
  ;[0 0 0] Take Photo
  (Utilities|FlowControl|Delay Delay)
  (Utilities|IsValid (CallFunction|GetSceneCapturer)
    (:Is%20Valid
      _)
    (:Is%20Not%20Valid
      (|CreateCaptureComponent)))
  (Transformation|SetWorldRotation (CallFunction|GetSceneCapturer) (|CalculateRotation TargetRotation TargetLocation TargetByRotation TargetActor) false false)
  (bind _returnvalue (Rendering|CreateRenderTarget2D 720 360 "RTF_RGBA8_SRGB"))
  (Variables|/Script/Engine.SceneCaptureComponent2D|SetTextureTarget _output _returnvalue)
  (Rendering|SceneCapture|CaptureScene _output :!class /Script/Engine.SceneCaptureComponent2D)
  (Variables|/Script/Engine.SceneCaptureComponent2D|SetTextureTarget _output 0)
  (Utilities|Array|Add _receivedphoto _returnvalue)
  (Default|SendMessage (Variables|Default|GetPlayerPhoneComponent) "" _npc_number _npc_number false (Utilities|Array|LastIndex _receivedphoto) false))

(event Custom|SendNPCToTarget
  (params (TargetActor :type Actor%20Object%20Reference) (AcceptanceRadius :type Float%20%28single-precision%29) (FollowMode :type Boolean) (FindDetails :type S%20Find%20Actor%20Details%20Structure))
  (bind _returnvalue (CallFunction|FindActor FindDetails))
  (bind _returnvalue_2 (Utilities|IsValid _returnvalue))
  (bind _returnvalue_3 (select _returnvalue_2 _returnvalue TargetActor))
  ;[0 0 0] Send Npc to Target
  (AI|AIMoveTo (Variables|Default|GetOwner) "0, 0, 0" _returnvalue_3 AcceptanceRadius false :!label _label
    (:OnSuccess
      (if FollowMode
        (Utilities|FlowControl|Delay 0.2)
        (Utilities|FlowControl|Sequence
          (:then_0
            (Utilities|FlowControl|Gate false
              (:Exit
                (goto _label))))
          (:then_1
            _)))
      (Default|CallNPCReachTarget _returnvalue_3))
    (:OnFail
      (Utilities|FlowControl|Delay 0.2)
      (Utilities|FlowControl|Gate false
        (:Exit
          (goto _label))))))

(event EventBeginPlay
  ;[0 0 0] Beginplay
  (bind _aspawn (Utilities|Casting|CastToPawn (Components|GetOwner)))
  (if (Pawn|IsPlayerControlled _aspawn)
    (Development|PrintString "only bots can use" true true "(R=1.000000,G=0.000000,B=0.000000,A=1.000000)")
    (Components|DestroyComponent)
    (else
      (Variables|Default|SetOwner _aspawn)
      (Variables|Default|SetAIController (AI|GetAIController (Variables|Default|GetOwner))))))

(fn FindActor
  (params (Details :type S%20Find%20Actor%20Details%20Structure))
  (bind (_class _tag _index) (Utilities|Struct|BreakS_FindActorDetails Details))
  (bind _outactors (Actor|GetAllActorsOfClasswithTag _class _tag))
  (return (select (Utilities|Array|IsValidIndex _outactors _index) (Utilities|Array|Get(acopy) _outactors _index) (Utilities|Array|Get(acopy) _outactors))))

(fn GetSceneCapturer
  (return (Utilities|Array|Get(acopy) (Actor|GetComponentsbyTag (Variables|Default|GetOwner) "/Script/Engine.SceneCaptureComponent2D" "PhotoCamera"))))