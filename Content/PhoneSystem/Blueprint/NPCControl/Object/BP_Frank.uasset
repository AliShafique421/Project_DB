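; BP_Frank is the phone-contact control object for NPC Frank, scripting his reactions to the player's texts, calls and money.
; Keyword-matched messages trigger replies, money, media, or sending his AI character to the player or a photo spot.
; Calls are answered with dialogue while OpenPhone is set, otherwise rejected with a random one-shot MultiGate follow-up.
; One follow-up chases the player, ragdolls them with an impulse and shows the death screen.
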(event Custom|CustomEvent
  (CallFunction|PlayDialogue (EventDispatchers|CreateEvent (CallFunction|GetDialogueComponent) :!event WrongNumberDialogue)))

(event EventdMoney
  (params (Amount :type Float%20%28double-precision%29))
  (CallFunction|SendMessage "thanks bro" 2.0 false))

(event EventdMessage
  (params (Message :type String))
  ;[0 0 0] Received Message
  (switch string (Utilities|String|ToLower Message)
    (:hi
      (CallFunction|SendMessage "Hello, who are you" 0.2 false :!label _label))
    (:hello
      (goto _label))
    (:can%20you%20spot%20me
      (CallFunction|SendMessage "okey" 0.2 false)
      (CallFunction|SendMoneytoPlayer 5e+01 2.0))
    (:come
      (CallFunction|SendNPCTarget :TargetActor (Components|GetOwner (CallFunction|GetComponentReferance)) :StartsDelay 2.0))
    (:go%20to%20photo
      (|CollapseGraph))
    (:send%20photo
      (CallFunction|SendPhototoPlayer "/Game/PhoneSystem/Demo/Texture/ProfilePicture/T_AngryMan.T_AngryMan" 2.0 false))
    (:send%20sound
      (Default|SendSoundPlayerwithDelay (CallFunction|GetComponentReferance) (Variables|Default|GetMyNumber) "/Game/PhoneSystem/Demo/Sound/Dialog/AngryMan/SW_WarnMessage.SW_WarnMessage" 0.0 false))))

(event EventIncomingCall
  (bind _component (CallFunction|GetComponentReferance))
  (if (Variables|Default|GetOpenPhone)
    (Default|OpenPhone (CallFunction|GetCallingScreen) 1.0 self)
    (EventDispatchers|BindEventtoDelayEnd (CallFunction|GetCallingScreen) (delegate Custom|CustomEvent))
    (else
      (Default|RejectPhone (CallFunction|GetCallingScreen) 1.0 "Busy..." "/Game/PhoneSystem/Sound/SW_Beep.SW_Beep")
      (Utilities|FlowControl|MultiGate true false -1
        (:Out%200
          (CallFunction|SendMessage "don't call me again" 3.0 false))
        (:Out%201
          (Default|SendSoundPlayerwithDelay (CallFunction|GetComponentReferance) (Variables|Default|GetMyNumber) "/Game/PhoneSystem/Demo/Sound/Dialog/AngryMan/SW_WarnMessage.SW_WarnMessage" 2.0 false))
        (:Out%202
          (Variables|Default|GetAICharacter
            (:then
              (CallFunction|SendMessage "I will beat you" 2.0 false)
              (CallFunction|SendNPCTarget :TargetActor (Components|GetOwner _component) :StartsDelay 2.0)
              (|ChasePlayer _component))
            (:else)))))))

(event EventPhoneClosedwithAnyReason
  (Variables|Default|SetOpenPhone false))

(event Custom|NPCReachTarget_Event
  (params (Actor :type Actor%20Object%20Reference))
  (bind _ascharacter (Utilities|Casting|CastToCharacter Actor))
  (EventDispatchers|UnbindEventfromNPCReachTarget (stale _self) (delegate Custom|NPCReachTarget_Event))
  (Pawn|Components|CharacterMovement|DisableMovement (Variables|/Script/Engine.Character|GetCharacterMovement _ascharacter))
  (Collision|SetCollisionEnabled (Variables|/Script/Engine.Character|GetMesh _ascharacter) "QueryAndPhysics")
  (Physics|SetSimulatePhysics (Variables|/Script/Engine.Character|GetMesh _ascharacter) true)
  (Physics|AddImpulse (Variables|/Script/Engine.Character|GetMesh _ascharacter) (* (Math|Vector|GetForwardVector (Math|Rotator|FindLookatRotation (Transformation|GetActorLocation (Variables|Default|GetAICharacter)) (Transformation|GetActorLocation _ascharacter))) 6e+04) "None" false)
  (Default|CreateDeadScreen (CallFunction|GetComponentReferance)))

(event Custom|CustomEvent_1
  (params (Actor :type Actor%20Object%20Reference))
  (EventDispatchers|UnbindEventfromNPCReachTarget (CallFunction|GetComponentReferance) (delegate Custom|CustomEvent_1))
  (bind _aicharacter (Variables|Default|GetAICharacter)
    (:then
      (Default|TakePhoto (Actor|GetComponentbyClass _aicharacter "/Game/PhoneSystem/Blueprint/NPCControl/AC_NPCActionComponent.AC_NPCActionComponent_C") "0, 0, 0" "0, 0, 0" false 0.2 Actor))
    (:else)))