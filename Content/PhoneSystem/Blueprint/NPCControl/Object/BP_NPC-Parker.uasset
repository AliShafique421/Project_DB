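; Phone-system control object for the NPC Parker, defining how he reacts to the player's messages, photos and calls.
; Matched text keywords trigger replies, money, photo or sound sends, or send his AI character to the player or off to photograph a tagged cube.
; Calls are either rejected as busy or answered with a dialogue.
; When the call closes, specific dialogue answers arm a photo request that pays the player for a correctly tagged photo.
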(event Custom|PlayDialogue1
  (CallFunction|PlayDialogue (EventDispatchers|CreateEvent (CallFunction|GetDialogueComponent) :!event ParkerDialogue)))

(event EventdMessage
  (params (Message :type String))
  ;[0 0 0] Received Message
  (switch string (Utilities|String|ToLower Message)
    (:hi
      (CallFunction|SendMessage "Hello, who are you" 0.2 false :!label _label))
    (:hello
      (goto _label))
    (:can%20you%20spot%20me
      (CallFunction|SendMessage "okey" 0.2 false)
      (CallFunction|SendMoneytoPlayer 5e+01 2.0))
    (:come
      (CallFunction|SendNPCTarget :TargetActor (Components|GetOwner (CallFunction|GetComponentReferance)) :StartsDelay 2.0))
    (:go%20to%20photo
      (|CollapseGraph_2))
    (:send%20photo
      (CallFunction|SendPhototoPlayer "/Game/PhoneSystem/Demo/Texture/ProfilePicture/T_AngryMan.T_AngryMan" 2.0 false))
    (:send%20sound
      (Default|SendSoundPlayerwithDelay (CallFunction|GetComponentReferance) (Variables|Default|GetMyNumber) "/Game/PhoneSystem/Demo/Sound/Dialog/AngryMan/SW_WarnMessage.SW_WarnMessage" 0.0 false))))

(event EventIncomingCall
  (bind _referance (CallFunction|GetCallingScreen))
  (if (Variables|Default|GetOpenPhone)
    (Default|OpenPhone _referance 1.0 self)
    (EventDispatchers|BindEventtoDelayEnd (CallFunction|GetCallingScreen) (delegate Custom|PlayDialogue1))
    (else
      (Default|RejectPhone _referance 2.0 "Busy..." "/Game/PhoneSystem/Sound/SW_Rejected.SW_Rejected"))))

(event EventdPhoto
  (params (PhotoTag :type String))
  (if (Variables|Default|GetWaitPhoto)
    (if (Utilities|Enum|Equal(Enum) PhotoTag "npccube")
      (CallFunction|SendMessage "Thanks bro. I'll send you some money." 1.0 false)
      (CallFunction|SendMoneytoPlayer 1e+02 2.0))))

(event EventPhoneClosedwithAnyReason
  (bind _returnvalue (Default|CheckAnswers (CallFunction|GetDialogueComponent) (Utilities|Array|MakeArray (Utilities|Struct|MakeS_DialogueAnswers) (Utilities|Struct|MakeS_DialogueAnswers 1))))
  (Variables|Default|SetWaitPhoto _returnvalue))

(event Custom|CustomEvent_1
  (params (Actor :type Actor%20Object%20Reference))
  (EventDispatchers|UnbindEventfromNPCReachTarget (CallFunction|GetComponentReferance) (delegate Custom|CustomEvent_1))
  (bind _aicharacter (Variables|Default|GetAICharacter)
    (:then
      (Default|TakePhoto (Actor|GetComponentbyClass _aicharacter "/Game/PhoneSystem/Blueprint/NPCControl/AC_NPCActionComponent.AC_NPCActionComponent_C") "0, 0, 0" "0, 0, 0" false 0.2 Actor))
    (:else)))