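; Phone control object for the NPC Finn, scripting how Finn reacts to the player's texts, photos and calls.
; Keyword messages trigger replies, a timed event or server-side movement to the player or a tagged photo spot, where arrival fires a photo action.
; Incoming calls either play dialogue after a pickup delay or are rejected as busy with a follow-up text.
; A finished call sends Finn to the player.
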(event Custom|CustomEvent
  (CallFunction|PlayDialogue (EventDispatchers|CreateEvent (CallFunction|GetDialogueComponent) :!event CallNPC)))

(event Custom|NPCReachTarget_Event
  (params (Actor :type Actor%20Object%20Reference))
  (EventDispatchers|UnbindEventfromNPCReachTarget (CallFunction|GetComponentReferance) (delegate Custom|NPCReachTarget_Event)))

(event Custom|CustomEvent_1
  (params (Actor :type Actor%20Object%20Reference))
  (EventDispatchers|UnbindEventfromNPCReachTarget (CallFunction|GetComponentReferance) (delegate Custom|CustomEvent_1))
  (bind _aicharacter (Variables|Default|GetAICharacter)
    (:then
      (Default|TakePhoto (Actor|GetComponentbyClass _aicharacter "/Game/PhoneSystem/Blueprint/NPCControl/AC_NPCActionComponent.AC_NPCActionComponent_C") "0, 0, 0" "0, 0, 0" false 0.2 Actor))
    (:else)))

(event EventdPhoto
  (params (PhotoTag :type String))
  (if (Utilities|Enum|Equal(Enum) PhotoTag "npccube")
    (CallFunction|SendMessage "looks good :)" 0.4 false)))

(event EventdMessage
  (params (Message :type String))
  (bind _component (CallFunction|GetComponentReferance))
  (bind _component_2 (CallFunction|GetComponentReferance))
  (switch string (Utilities|String|ToLower Message)
    (:go%20to%20photo
      (CallFunction|SendMessage "okey" 0.2 false)
      (Default|SendNPCtoTargetServer _component_2 (Actor|GetComponentbyClass (Variables|Default|GetAICharacter) "/Game/PhoneSystem/Blueprint/NPCControl/AC_NPCActionComponent.AC_NPCActionComponent_C") 0 3.5e+02 false (Utilities|Struct|MakeS_FindActorDetails "/Script/Engine.StaticMeshActor" "Photo_Cube") 0.0)
      (EventDispatchers|BindEventtoNPCReachTarget _component_2 (delegate Custom|CustomEvent_1)))
    (:come
      (CallFunction|SendMessage "okey" 0.2 false)
      (Default|SendNPCtoTargetServer :self _component :NPCActionComponent (Actor|GetComponentbyClass (Variables|Default|GetAICharacter) "/Game/PhoneSystem/Blueprint/NPCControl/AC_NPCActionComponent.AC_NPCActionComponent_C") :TargetActor (Components|GetOwner _component) :AcceptanceRadius 5e+01)
      (EventDispatchers|AssignNPCReachTarget _component (delegate Custom|NPCReachTarget_Event)))
    (:call%20me
      (Utilities|Time|SetTimerbyEvent (EventDispatchers|CreateEvent :!event CallPlayer) 0.3))
    (:hi
      (CallFunction|SendMessage "hi" 0.2 false))))

(event EventIncomingCall
  (bind _referance (CallFunction|GetCallingScreen))
  (if (Variables|Default|GetOpenPhone)
    (Default|OpenPhone _referance 1.0 self)
    (EventDispatchers|BindEventtoDelayEnd (CallFunction|GetCallingScreen) (delegate Custom|CustomEvent))
    (else
      (Default|RejectPhone _referance 2.0 "Busy..." "/Game/PhoneSystem/Sound/SW_Beep.SW_Beep")
      (CallFunction|SendMessage "I'm not available right now" 2.0 false))))

(event EventPlayerCallRejected
  (|CallParentFunction)
  (CallFunction|SendMessage "don't you want to talk to me" 1.0 false))

(event EventClosePhone
  (params (Finished :type Boolean))
  (bind _component (CallFunction|GetComponentReferance))
  (|CallParentFunction Finished)
  (if Finished
    (Default|SendNPCtoTargetServer :self _component :NPCActionComponent (Actor|GetComponentbyClass (Variables|Default|GetAICharacter) "/Game/PhoneSystem/Blueprint/NPCControl/AC_NPCActionComponent.AC_NPCActionComponent_C") :TargetActor (Components|GetOwner _component) :AcceptanceRadius 5e+01)))