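; Dialogue component for the phone system that runs scripted NPC conversations, written here as event chains such as WrongNumberDialogue and ParkerDialogue.
; StartDialogue creates the dialogue widget and binds its input; End and Stop events handle teardown and notify listeners.
; Speak and GivePlayerOptions macros poll with delay loops for input or closure, with voiced lines also auto-advancing after the sound's duration.
; Chosen options are recorded for CheckAnswers until EndDialogue clears them.
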(event Custom|TestCall
  (CallFunction|StartDialogue)
  (Utilities|Speak "Hi bro" 0 true
    (:Next
      (Utilities|Speak "Hi" 0 false
        (:Next
          (bind _selectedindex (Utilities|GivePlayerOptions "Do you like this asset?" (Utilities|Array|MakeArray "Yes,definitely." "No, it has problems or shortcomings."))
            (:Next
              (switch int _selectedindex
                (:0
                  (bind _selectedindex_2 (Utilities|GivePlayerOptions "I'm glad to hear that, how about you check out my other assets?" (Utilities|Array|MakeArray "yes i want" "No, I don't have time for that."))
                    (:Next
                      (switch int _selectedindex_2
                        (:0
                          (Utilities|Speak "You can check out Sametstore products via Fab." 0 true
                            (:Next
                              _)))
                        (:1
                          (Utilities|Speak "okey" 0 true
                            (:Next
                              _))))
                      (Utilities|Speak "see you later" 0 true
                        (:Next
                          (CallFunction|EndDialogue))))))
                (:1
                  (Utilities|Speak "I'm sorry to hear that, we'll make improvements as soon as possible." 0 true
                    (:Next
                      (Utilities|Speak "see you later" 0 true
                        (:Next
                          (CallFunction|EndDialogue))))))))))))))

(event Custom|WrongNumberDialogue
  (CallFunction|StartDialogue)
  (Utilities|Speak "Hello, who are you?" "/Game/PhoneSystem/Demo/Sound/Dialog/AngryMan/SW_001.SW_001" true
    (:Next
      (Utilities|Speak "Hi, this is Pops. I think I dialed the wrong number." "/Game/PhoneSystem/Demo/Sound/Dialog/AngryMan/Player/SW_001.SW_001" true
        (:Next
          (Utilities|Speak "What are you doing at this hour? Who is this Pops?" "/Game/PhoneSystem/Demo/Sound/Dialog/AngryMan/SW_002.SW_002" true
            (:Next
              (Utilities|Speak "I'm sorry, good evening." "/Game/PhoneSystem/Demo/Sound/Dialog/AngryMan/Player/SW_002.SW_002" true
                (:Next
                  (Utilities|Speak "Don't ever call me again!" "/Game/PhoneSystem/Demo/Sound/Dialog/AngryMan/SW_003.SW_003" true
                    (:Next
                      (CallFunction|EndDialogue))))))))))))

(event Custom|ClosedDialogueEvent
  ;[0 0 0] Dialogue Closed
  (bind _dialoguewidget (Variables|Default|GetDialogueWidget)
    (:then
      (EventDispatchers|UnbindallEventsfromNext _dialoguewidget)
      (EventDispatchers|UnbindallEventsfromSelectedOptions _dialoguewidget)
      (Variables|Default|SetSelectedOptions -1)
      (Variables|Default|SetQuestion false)
      (Variables|Default|SetCanNext false)
      (Variables|Default|SetCurrentPlayDialogue false))
    (:else
      _))
  (Widget|RemovefromParent _dialoguewidget)
  (Variables|Default|SetDialogueWidget 0))

(event Custom|Next_Event
  ;[0 0 0] Start Dialogue
  (if (not (Variables|Default|GetQuestion))
    (Variables|Default|SetCanNext true)))

(event Custom|SelectedOptions_Event
  (params (Index :type Integer))
  ;[0 0 0] Start Dialogue
  (Variables|Default|SetSelectedOptions Index)
  (Variables|Default|SetCanNext true))

(event Custom|EndDialogue
  ;[0 0 0] End Dialogue
  (bind _dialoguewidget (Variables|Default|GetDialogueWidget)
    (:then
      (EventDispatchers|UnbindallEventsfromNext _dialoguewidget)
      (EventDispatchers|UnbindallEventsfromSelectedOptions _dialoguewidget)
      (Variables|Default|SetSelectedOptions -1)
      (Variables|Default|SetQuestion false)
      (Variables|Default|SetCanNext false)
      (Variables|Default|SetCurrentPlayDialogue false))
    (:else
      _))
  (Widget|RemovefromParent _dialoguewidget)
  (Variables|Default|SetDialogueWidget 0)
  (Default|CallOnEndDialogue)
  (Utilities|FlowControl|Delay 0.2)
  (Utilities|Array|Clear (Variables|Default|GetSelectedOptionsList)))

(event Custom|StartDialogue
  ;[0 0 0] Start Dialogue
  (Variables|Default|SetCurrentPlayDialogue true)
  (bind _returnvalue (UserInterface|CreateWidget "/Game/PhoneSystem/Blueprint/Dialogue/WBP_DialogueSystemBase.WBP_DialogueSystemBase_C"))
  (UserInterface|Viewport|AddtoPlayerScreen _returnvalue)
  (bind _output_get (Variables|Default|SetDialogueWidget _returnvalue))
  (EventDispatchers|AssignNext _output_get (delegate Custom|Next_Event))
  (EventDispatchers|AssignSelectedOptions _output_get (delegate Custom|SelectedOptions_Event))
  (Variables|Default|SetDialogueClosed false)
  (Variables|Default|SetCanNext false)
  (Variables|Default|SetSelectedOptions -1)
  (Default|CallOnDialogueStarted))

(event Custom|CallNPC
  (CallFunction|StartDialogue)
  (Utilities|Speak "Finn, where are you  ?" "/Game/PhoneSystem/Demo/Sound/Dialog/CallNPC/Player/SW_001.SW_001" false
    (:Next
      (Utilities|Speak "I was resting, what happened?" "/Game/PhoneSystem/Demo/Sound/Dialog/CallNPC/SW_001.SW_001" true
        (:Next
          (Utilities|Speak "come to me immediately" "/Game/PhoneSystem/Demo/Sound/Dialog/CallNPC/Player/SW_002.SW_002" false
            (:Next
              (Utilities|Speak "Okay, I am coming" "/Game/PhoneSystem/Demo/Sound/Dialog/CallNPC/SW_002.SW_002" true
                (:Next
                  (CallFunction|EndDialogue))))))))))

(event Custom|ParkerDialogue
  (CallFunction|StartDialogue)
  (Utilities|Speak "Hi" 0 true
    (:Next
      (Utilities|Speak "Hi" 0 false
        (:Next
          (bind _selectedindex (Utilities|GivePlayerOptions "I've got a great gig. Wanna join?" (Utilities|Array|MakeArray "What's the deal?" "No, I've got things to take care of."))
            (:Next
              (switch int _selectedindex
                (:0
                  (bind _selectedindex_2 (Utilities|GivePlayerOptions "I've heard there's a blue cube in Maplewood. I'd like you to take a picture of it for me." (Utilities|Array|MakeArray "Sure, I'll send the photo as a message." "No, I've got things to take care of."))
                    (:Next
                      (switch int _selectedindex_2
                        (:0
                          (Utilities|Speak "Thanks, buddy. I'm waiting." 0 true
                            (:Next
                              (Utilities|Speak "okey" 0 false
                                (:Next
                                  _)))))
                        (:1
                          (Utilities|Speak "Alright, it's up to you. Take care!" 0 true
                            (:Next
                              (Utilities|Speak "See you later!" 0 false
                                (:Next
                                  _))))))
                      (CallFunction|EndDialogue))))
                (:1
                  (Utilities|Speak "Alright, it's up to you. Take care!" 0 true
                    (:Next
                      (Utilities|Speak "See you later!" 0 false
                        (:Next
                          (CallFunction|EndDialogue))))))))))))))

(event Custom|StopDialogue
  ;[0 0 0] Close Dialogue
  (if (Variables|Default|GetCurrentPlayDialogue)
    (Variables|Default|SetDialogueClosed true)
    (Variables|Default|SetCurrentPlayDialogue false)
    (Default|CallOnDialogueStopped)))

(fn CheckAnswers
  (params (Question/Answer :type Array%20of%20S%20Dialogue%20Answers%20Structures))
  (if (>= (Utilities|Array|Length (Variables|Default|GetSelectedOptionsList)) (Utilities|Array|Length Question/Answer))
    (for _array_element Question/Answer
      (if (not (== (Utilities|Array|Get(acopy) (Variables|Default|GetSelectedOptionsList) (.QuestionIndex (Utilities|Struct|BreakS_DialogueAnswers _array_element))) (.AnswerIndex (Utilities|Struct|BreakS_DialogueAnswers _array_element))))
        (return false)))
    (return true)
    (else
      (return false))))