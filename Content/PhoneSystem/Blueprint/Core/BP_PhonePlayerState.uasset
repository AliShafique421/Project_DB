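; Player state for a multiplayer in-game phone, carrying each player's profile, per-number message history and call status.
; It auto-registers on BeginPlay with a server or random client number; replication then adds the profile as a contact.
; Messages, deletions and voice/video call signals go through server events that find the target by number in PlayerArray and invoke its owning-client events.
; Those events drive the WBP_MainPhone apps and notifications, while CanCall handles busy rejection.
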(event Custom|SetProfileDetails_Server
  (params (Name :type String) (Number :type String) (ProfileIcon :type Texture%202D%20Object%20Reference))
  ;[0 0 0] Set Profile Details (Server)
  (Variables|Profile|SetProfileDetails (Utilities|Struct|MakeS_ProfileDetails Name Number ProfileIcon))
  (Variables|Profile|SetIsRegistered true))

(event Custom|ReceivedMessage
  (params (SenderNumber :type String%20%28by%20ref%29) (MessageDetails :type S%20Message%20Data%20Structure))
  ;[0 0 0] Messaging
  (Message|AddMessageList SenderNumber MessageDetails)
  (Message|ReceivedReplayedMessage MessageDetails))

(event Custom|CantCallSomeone_OwningClient
  (params (ReceiverNumber :type String) (Video :type Boolean))
  (bind _output (Other|GetWidgetRef))
  (bind _currentappref (Variables|/Game/PhoneSystem/UI/WBP_MainPhone.WBP_MainPhone_C|GetCurrentAppRef _output))
  ;[0 0 0] Calling| Caller Events
  (CallFunction|SetCallParameterServer true false)
  (if Video
    (bind _aswbp_video_chats (Utilities|Casting|CastToWBP_VideoChats _currentappref))
    (Default|RejectPhone _aswbp_video_chats "Busy..." "/Game/PhoneSystem/Sound/SW_Rejected.SW_Rejected")
    (else
      (bind _aswbp_calling_page (Utilities|Casting|CastToWBP_CallingPage _currentappref))
      (Default|RejectPhone _aswbp_calling_page 0.0 "Busy..." "/Game/PhoneSystem/Sound/SW_Rejected.SW_Rejected"))))

(event Custom|ForwardCall_Server
  (params (ReceiverNumber :type String) (CallerNumber :type String) (Video :type Boolean))
  (bind _returnvalue (Other|FindPlayerStatefromNumber ReceiverNumber))
  ;[0 0 0] Call Server Event
  (Utilities|IsValid _returnvalue
    (:Is%20Valid
      (if (Variables|BP_PhonePlayerState_C|GetCanCall _returnvalue)
        (CallFunction|ReceiveCallOwningClient _returnvalue CallerNumber Video)
        (else
          (CallFunction|CantCallSomeoneOwningClient (Other|FindPlayerStatefromNumber CallerNumber) ReceiverNumber Video :!label _label))))
    (:Is%20Not%20Valid
      (goto _label))))

(event Custom|SetCallParameter_Server
  (params (CanCall :type Boolean) (OnVideoCall :type Boolean))
  ;[0 0 0] Call Server Event
  (bind _output_get (Variables|Call|SetCanCall CanCall))
  (if _output_get
    (Variables|Default|SetOnVideoCall OnVideoCall)
    (else
      (Variables|Default|SetOnVideoCall false))))

(event Custom|ForwardMessageDeleted_Server
  (params (DeleterPhoneNumber :type String) (ReceiverNumber :type String) (DeletedMessageIndex :type Integer))
  ;[0 0 0] Messaging
  (CallFunction|OnMessageDeletedOwningClient (Other|FindPlayerStatefromNumber ReceiverNumber) DeleterPhoneNumber DeletedMessageIndex))

(event Custom|OtherPlayerAnswerCall_OwningClient
  (params (Open :type Boolean) (ReceiverNumber :type String) (Video :type Boolean))
  ;[0 0 0] Calling| Caller Events
  (if Video
    (|AnswerCallVideo Open)
    (else
      (|AnswerCallVoice Open))))

(event Custom|ToggleCamera_OwningClient
  ;[0 0 0] Video Chat
  (bind _aswbp_video_chats (Utilities|Casting|CastToWBP_VideoChats (Variables|/Game/PhoneSystem/UI/WBP_MainPhone.WBP_MainPhone_C|GetCurrentAppRef (Other|GetWidgetRef))))
  (Default|ToggleCamera _aswbp_video_chats))

(event Custom|Fix
  (bind _profiledetails (Variables|Profile|GetProfileDetails))
  (bind (_name _number) (Utilities|Struct|BreakS_ProfileDetails _profiledetails))
  (Utilities|FlowControl|Delay 0.2 :!label _label)
  (if (Variables|Profile|GetAutoAddContact)
    (bind _foundwidgets (Widget|GetAllWidgetsOfClass "/Game/PhoneSystem/UI/WBP_MainPhone.WBP_MainPhone_C" false))
    (Utilities|IsValid (Utilities|Array|Get(acopy) _foundwidgets)
      (:Is%20Valid
        (Default|AddNewContact (Utilities|Array|Get(acopy) _foundwidgets) _number _name))
      (:Is%20Not%20Valid
        (Utilities|FlowControl|DoOnce false
          (:Completed
            (goto _label)))))))

(event Custom|ForwardCloseVoiceCall_Server
  (params (OtherPlayerNumber :type String) (YourNumber :type String) (CallOpened :type Boolean) (Video :type Boolean))
  (bind _returnvalue (Other|FindPlayerStatefromNumber OtherPlayerNumber))
  ;[0 0 0] Call Server Event
  (Utilities|IsValid _returnvalue
    (:Is%20Valid
      (CallFunction|CallClosedOwningClient _returnvalue YourNumber CallOpened Video))))

(event Custom|OnMessageDeleted_OwningClient
  (params (DeleterPhoneNumber :type String) (DeletedMessageIndex :type Integer))
  ;[0 0 0] Messaging
  (CallFunction|RemoveMessage DeleterPhoneNumber DeletedMessageIndex true))

(event Custom|CallClosed_OwningClient
  (params (OtherPlayerNumber :type String) (CallOpened :type Boolean) (Video :type Boolean))
  ;[0 0 0] Calling Receiver Events
  (if Video
    (|CallClosed_Video CallOpened)
    (else
      (|CallClosed_Voice CallOpened))))

(event Custom|CloseCall_OwningClient
  (params (OtherPlayerNumber :type String) (CallOpened :type Boolean) (Video :type Boolean))
  ;[0 0 0] Calling Receiver Events
  (CallFunction|ForwardCloseVoiceCallServer OtherPlayerNumber (Utilities|Struct|BreakS_ProfileDetails (Variables|Profile|GetProfileDetails)) CallOpened Video)
  (CallFunction|SetCallParameterServer true false))

(event Custom|SendMessage
  (params (ReceiverNumber :type String) (MessageDetails :type S%20Message%20Data%20Structure%20%28by%20ref%29))
  ;[0 0 0] Messaging
  (Message|AddMessageList ReceiverNumber MessageDetails)
  (CallFunction|ForwardMessageServer ReceiverNumber MessageDetails (Utilities|Struct|BreakS_ProfileDetails (Variables|Profile|GetProfileDetails))))

(event Custom|SetOnline
  (params (Online :type Boolean))
  ;[0 0 0] Messaging
  (Variables|Default|SetIsMessageOnline Online))

(event Custom|ForwardMessage_Server
  (params (ReceiverNumber :type String) (MessageDetails :type S%20Message%20Data%20Structure%20%28by%20ref%29) (SenderNumber :type String))
  ;[0 0 0] Messaging
  (CallFunction|ReceivedMessage (Other|FindPlayerStatefromNumber ReceiverNumber) SenderNumber MessageDetails))

(event Custom|CallSomeone_OwningClient
  (params (Number :type String) (Video :type Boolean))
  ;[0 0 0] Calling| Caller Events
  (if (Variables|Call|GetCanCall)
    (CallFunction|ForwardCallServer Number (Utilities|Struct|BreakS_ProfileDetails (Variables|Profile|GetProfileDetails)) Video)
    (CallFunction|SetCallParameterServer false Video)))

(event Custom|AnswerCallForward_Server
  (params (Open :type Boolean) (CallerNumber :type String) (ReceiverNumber :type String) (Video :type Boolean))
  (bind _returnvalue (Other|FindPlayerStatefromNumber CallerNumber))
  ;[0 0 0] Call Server Event
  (Utilities|IsValid _returnvalue
    (:Is%20Valid
      (CallFunction|OtherPlayerAnswerCallOwningClient _returnvalue Open ReceiverNumber Video))))

(event Custom|ForwardToggleCamera_Server
  (params (Number :type String))
  (bind _returnvalue (Other|FindPlayerStatefromNumber Number))
  ;[0 0 0] Video Chat
  (Utilities|IsValid _returnvalue
    (:Is%20Valid
      (CallFunction|ToggleCameraOwningClient _returnvalue))))

(event Custom|AnswerCall_OwningClient
  (params (Open :type Boolean) (CallerNumber :type String) (Video :type Boolean))
  ;[0 0 0] Calling Receiver Events
  (CallFunction|AnswerCallForwardServer Open CallerNumber (Utilities|Struct|BreakS_ProfileDetails (Variables|Profile|GetProfileDetails)) Video)
  (CallFunction|SetCallParameterServer (not Open) Video))

(event EventBeginPlay
  ;[0 0 0] Beginplay
  (if (Class|KismetSystemLibrary|MakeLiteralBool true)
    (Other|AutoRegister)))

(fn ConstructionScript)

(fn OnRepIsRegistered
  (bind _profiledetails (Variables|Profile|GetProfileDetails))
  (bind (_name _number) (Utilities|Struct|BreakS_ProfileDetails _profiledetails))
  (if (Variables|Profile|GetAutoAddContact)
    (bind _foundwidgets (Widget|GetAllWidgetsOfClass "/Game/PhoneSystem/UI/WBP_MainPhone.WBP_MainPhone_C" false))
    (if (Utilities|Array|IsNotEmpty _foundwidgets)
      (Utilities|IsValid (Utilities|Array|Get(acopy) _foundwidgets)
        (:Is%20Valid
          (Default|AddNewContact (Utilities|Array|Get(acopy) _foundwidgets) _number _name))
        (:Is%20Not%20Valid
          (CallFunction|Fix))))))

(fn AutoRegister
  (bind _returnvalue (Math|Random|RandomIntegerinRange 1000 10000))
  (bind _returnvalue_2 (Utilities|String|ToString(Integer) _returnvalue))
  (bind _asplayer_controller (Utilities|Casting|CastToPlayerController (Components|GetOwner)))
  (if (Pawn|IsLocalController _asplayer_controller)
    (if (Networking|IsServer)
      (CallFunction|SetProfileDetailsServer "server" "000" "/Game/PhoneSystem/Demo/Texture/ProfilePicture/T_NewProfilePhoto.T_NewProfilePhoto")
      (else
        (CallFunction|SetProfileDetailsServer (Utilities|String|Append "Client" _returnvalue_2) _returnvalue_2 "/Game/PhoneSystem/Demo/Texture/ProfilePicture/T_NewProfilePhoto.T_NewProfilePhoto")))))

(fn AddMessageList
  (params (Receiver :type String%20%28by%20ref%29) (MessageData :type S%20Message%20Data%20Structure%20%28by%20ref%29))
  (bind _messagelist (Variables|Message|GetMessageList))
  (bind (_value _returnvalue) (Utilities|Map|Find _messagelist Receiver))
  (if _returnvalue
    (LocalVariables|SetOldMessage (Utilities|Struct|BreakS_MessageDetails _value)))
  (Utilities|Map|Remove (Variables|Message|GetMessageList) Receiver)
  (Utilities|Array|Add (LocalVariables|GetOldMessage) MessageData)
  (Utilities|Map|Add (Variables|Message|GetMessageList) Receiver (Utilities|Struct|MakeS_MessageDetails (LocalVariables|GetOldMessage))))

(fn FindPlayerStatefromNumber
  (params (Number :type String))
  (for _array_element (Variables|/Script/Engine.GameStateBase|GetPlayerArray (Game|GetGameState))
    (bind _asbp_phone_player_state (Utilities|Casting|CastToBP_PhonePlayerState _array_element))
    (if (Utilities|Enum|Equal(Enum) (Utilities|Struct|BreakS_ProfileDetails (Variables|BP_PhonePlayerState_C|GetProfileDetails _asbp_phone_player_state)) Number)
      (return _asbp_phone_player_state))))

(fn ReceivedReplayedMessage
  (params (MessageData :type S%20Message%20Data%20Structure))
  (bind _output (Other|GetWidgetRef))
  (bind _sendernumber (Utilities|Struct|BreakS_MessageData MessageData))
  (Utilities|IsValid _output
    (:Is%20Valid
      (if (Utilities|Enum|Equal(Enum) (Default|GetCurrentApp _output) "NewEnumerator5")
        (bind _aswbp_message_app (Utilities|Casting|CastToWBP_MessageApp (Variables|/Game/PhoneSystem/UI/WBP_MainPhone.WBP_MainPhone_C|GetCurrentAppRef _output)))
        (if (== (Class|WidgetSwitcher|GetActiveWidgetIndex (Variables|/Game/PhoneSystem/UI/Apps/WBP_MessageApp.WBP_MessageApp_C|GetWidgetSwitcher _aswbp_message_app)) 1)
          (if (Utilities|Enum|Equal(Enum) (Variables|/Game/PhoneSystem/UI/Apps/WBP_MessageApp.WBP_MessageApp_C|GetCurrentMessagingNumber _aswbp_message_app) _sendernumber)
            (Default|ReceivedReplayedMessage _aswbp_message_app MessageData)
            (else
              (if (Utilities|Enum|Equal(Enum) _sendernumber (Variables|/Game/PhoneSystem/UI/Apps/WBP_MessageApp.WBP_MessageApp_C|GetLastMessagingNumber _aswbp_message_app))
                (Default|ReceivedReplayedMessage _aswbp_message_app MessageData))
              (Message|Notify MessageData)))
          (else
            (Message|Notify MessageData)))
        (else
          (Message|Notify MessageData))))))

(fn Notify
  (params (MessageData :type S%20Message%20Data%20Structure))
  (bind _output (Other|GetWidgetRef))
  (bind (_message _date _sendernumber) (Utilities|Struct|BreakS_MessageData MessageData))
  (bind _mainscreenref (Variables|/Game/PhoneSystem/UI/WBP_MainPhone.WBP_MainPhone_C|GetMainScreenRef _output))
  (bind _returnvalue (Default|FindPlayerStatefromNumber _output _sendernumber))
  (bind (_find _details) (Default|GetProfleDetails _output _sendernumber))
  (bind (_name _number _profileicon) (Utilities|Struct|BreakS_ProfileDetails _details))
  (Audio|PlaySound2D "/Game/PhoneSystem/Demo/Sound/SW_Notify.SW_Notify" 1.0 1.0 0.0 0 0)
  (if _find
    (Default|NotifyMessage _mainscreenref _name _message _sendernumber _profileicon)
    (else
      (Utilities|IsValid _returnvalue
        (:Is%20Valid
          (Default|NotifyMessage _mainscreenref _sendernumber _message _sendernumber (Utilities|Struct|BreakS_ProfileDetails (Variables|BP_PhonePlayerState_C|GetProfileDetails _returnvalue))))))))

(fn GetWidgetRef
  (bind _foundwidgets (Widget|GetAllWidgetsOfClass "/Game/PhoneSystem/UI/WBP_MainPhone.WBP_MainPhone_C" false))
  (Utilities|IsValid (Utilities|Array|Get(acopy) _foundwidgets)
    (:Is%20Valid
      _)
    (:Is%20Not%20Valid
      _))
  (return (Utilities|Array|Get(acopy) _foundwidgets)))

(fn DeleteEmptyMessage
  (bind _messagelist (Variables|Message|GetMessageList))
  (bind _keys (Utilities|Map|Keys _messagelist))
  (for (_array_element _array_index) _keys
    (if (Utilities|Array|IsEmpty (Utilities|Struct|BreakS_MessageDetails (.Value (Utilities|Map|Find _messagelist _array_element))))
      (Utilities|Map|Remove _messagelist _array_element)
      (Utilities|Array|AddUnique (LocalVariables|GetNewLocalVar_0) _array_index)))
  (return (LocalVariables|GetNewLocalVar_0)))

(fn RemoveMessage
  (params (Number :type String) (MessageIndex :type Integer) (Forwarded :type Boolean))
  (LocalVariables|SetOldMessages (.messagelist (.Value (Utilities|Map|Find (Variables|Message|GetMessageList) Number))))
  (Utilities|Map|Remove (Variables|Message|GetMessageList) Number)
  (Utilities|Array|RemoveIndex (LocalVariables|GetOldMessages) MessageIndex)
  (Utilities|Map|Add (Variables|Message|GetMessageList) Number (Utilities|Struct|MakeS_MessageDetails (LocalVariables|GetOldMessages)))
  (if Forwarded
    (bind _aswbp_message_app (Utilities|Casting|CastToWBP_MessageApp (Variables|/Game/PhoneSystem/UI/WBP_MainPhone.WBP_MainPhone_C|GetCurrentAppRef (Other|GetWidgetRef))))
    (Default|OtherPlayerDeleteMessage _aswbp_message_app MessageIndex)
    (else
      (CallFunction|ForwardMessageDeletedServer (Utilities|Struct|BreakS_ProfileDetails (Variables|Profile|GetProfileDetails)) Number MessageIndex))))

(event Custom|ReceiveCall_OwningClient
  (params (CallerNumber :type String) (Video :type Boolean))
  (bind _output (Other|GetWidgetRef))
  (CallFunction|SetCallParameterServer false Video)
  (if (Variables|/Game/PhoneSystem/UI/WBP_MainPhone.WBP_MainPhone_C|GetIsPhoneOpen _output)
    _
    (else
      (Default|TogglePhone (Variables|/Game/PhoneSystem/UI/WBP_MainPhone.WBP_MainPhone_C|GetMainScreenRef _output) false false)))
  (if Video
    (bind _appreferance (Default|OpenApp (Other|GetWidgetRef) "NewEnumerator23" false))
    (bind _aswbp_video_chats (Utilities|Casting|CastToWBP_VideoChats _appreferance))
    (Default|SetUserDetails _aswbp_video_chats CallerNumber true)
    (else
      (bind _appreferance_2 (Default|OpenApp (Other|GetWidgetRef) "NewEnumerator20" false))
      (bind _aswbp_receive_call (Utilities|Casting|CastToWBP_ReceiveCall _appreferance_2))
      (Default|SetUserDetails _aswbp_receive_call CallerNumber 0 true))))