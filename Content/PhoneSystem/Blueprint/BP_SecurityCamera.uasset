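; BP_SecurityCamera is a remotely controllable security camera in the phone system, with pan, tilt, zoom and a can-connect flag.
; Server events clamp zoom, map it to scene capture FOV on the owning client, and scale sensitivity down as zoom increases.
; Movement input is scaled by that sensitivity and angle-clamped on the server, then multicast to rotate the pivot using roll and pitch.
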(event Custom|SetConnect_Server
  (params (CanConnect :type Boolean))
  ;[0 0 0] Can Connect
  (Variables|Default|SetCanConnect CanConnect))

(event Custom|MoveCamera_Server
  (params (Axis :type Vector%202D%20Structure))
  (bind (_x _y) (Math|Vector2D|BreakVector2D Axis))
  (bind _pivot (Variables|Default|GetPivot))
  (bind _relativerotation (Variables|/Script/Engine.SceneComponent|GetRelativeRotation _pivot))
  ;[0 0 0] Rotate Camera
  (CallFunction|SetCameraPositionMC (Math|Float|ClampAngle (+ (* (Variables|Default|GetSensitivity) _x) (.roll _relativerotation)) -9e+01 9e+01) (Math|Float|ClampAngle (+ (* _y (Variables|Default|GetSensitivity)) (.pitch _relativerotation)) -87.0 87.0)))

(event Custom|ZoomCamera_Server
  (params (Zoom :type Float%20%28double-precision%29))
  ;[0 0 0] Zoom Camera
  (bind _output_get (Variables|Default|SetZoom (Math|Float|Clamp(Float) (+ Zoom (Variables|Default|GetZoom)) 0.0 1e+02)))
  (CallFunction|SetFieldOfViewOwningClient (Math|Float|MapRangeClamped _output_get 0.0 1e+02 9e+01 1e+01))
  (Variables|Default|SetSensitivity (Math|Float|MapRangeClamped (Variables|Default|GetZoom) 0.0 1e+02 1.0 0.05)))

(event Custom|SetCameraPosition_MC
  (params (New%20Rotation%20X%20%28Roll%29 :type Float%20%28single-precision%29) (New%20Rotation%20Y%20%28Pitch%29 :type Float%20%28single-precision%29))
  ;[0 0 0] Rotate Camera
  (Transformation|SetRelativeRotation (Variables|Default|GetPivot) (Math|Rotator|MakeRotator New%20Rotation%20X%20%28Roll%29 New%20Rotation%20Y%20%28Pitch%29 0.0) false false))

(event Custom|SetFieldOfView_OwningClient
  (params (Field%20of%20View :type Float%20%28single-precision%29))
  ;[0 0 0] Zoom Camera
  (Variables|/Script/Engine.SceneCaptureComponent2D|SetFOVAngle (Variables|Default|GetSceneCaptureComponent2D) Field%20of%20View))

(fn ConstructionScript)